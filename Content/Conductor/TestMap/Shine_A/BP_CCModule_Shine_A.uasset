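; BP_CCModule_Shine_A is a Content Conductor module for the Shine_A test map that moves an NPC during Phase2.
; Phase entry sets a flag that is true only in Phase2.
; While it is set, each tick looks up managed actor ShineA_Npc_000 and offsets it along world X without sweep.
; The offset takes the sine of frame delta rather than elapsed time, producing a steady drift instead of oscillation.
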(event `self.OnTick`
  (params (DeltaSeconds :type "Float (single-precision)"))
  (if (`self.bIsPhase2`)
    (bind _returnvalue (`ContentConductor.FindManagedActor` (`self.GetContentConductor`) "ShineA_Npc_000"))
    (`/Engine/EditorBlueprintResources/StandardMacros.IsValid` _returnvalue
      (:`Is Valid`
        (`Actor.K2_SetActorLocation` _returnvalue (+ (`Actor.K2_GetActorLocation` _returnvalue) (`KismetMathLibrary.MakeVector` (* (`KismetMathLibrary.DegSin` (* DeltaSeconds 1.0)) 1000.0))) false false)))))

(event `self.OnEnterPhase`
  (params (Phase :type Name))
  (set `self.bIsPhase2` (== Phase "Phase2")))